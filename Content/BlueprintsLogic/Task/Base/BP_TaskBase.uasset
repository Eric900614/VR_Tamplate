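; Base task Blueprint for a hierarchical task system in a VR game, tracking child tasks and owned task items.
; On BeginPlay it registers with parent tasks and claims its items.
; While open, it recounts completed children and items, becoming complete when all are done.
; The TaskState RepNotify then notifies items and parents, broadcasts completion through GS_VR and opens closed related tasks, which check their own completion.
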(event Custom|InitTaskData
  (bind _taskitems (Variables|Config|GetTaskItems))
  ;[1 1 1] 统计子任务个数&任务物品个数
  (Utilities|FlowControl|Sequence
    (:then_0
      (Variables|Default|SetTaskItem_Count (Utilities|Array|Length _taskitems))
      (for _array_element (Variables|Config|GetParentTasks)
        (CallFunction|AddChildTask _array_element self)))
    (:then_1
      ;[1 1 1] 设置任务物品owner
      (for _array_element_2 _taskitems
        (Default|ServerSetOwner _array_element_2 self)))))

(event Custom|CheckChildTaskFinished
  ;[1 1 1] 更新子任务状态
  (if (CallFunction|IsOpenedTask)
    (Variables|Default|SetCompletedChildTask_Count 0)
    (for _array_element (Variables|Config|GetChildTasks)
      (if (Utilities|Enum|Equal(Enum) (Variables|BP_TaskBase_C|GetTaskState _array_element) "NewEnumerator2")
        (Math|Integer|IncrementInt (Variables|Default|GetCompletedChildTask_Count))))
    (CallFunction|CheckTaskState)))

(event Custom|CalculateCompletedTaskItemCount
  ;[1 1 1] 查看任务物品状态
  (Variables|Default|SetCompletedTaskItems_Count 0)
  (for _array_element (Variables|Config|GetTaskItems)
    (if (Utilities|Enum|Equal(Enum) (Variables|/Game/BlueprintsLogic/Task/Base/BP_TaskItemBase.BP_TaskItemBase_C|GetTaskItemRunningState _array_element) "NewEnumerator2")
      (Math|Integer|IncrementInt (Variables|Default|GetCompletedTaskItems_Count))))
  (CallFunction|CheckTaskState))

(event Custom|CheckTaskState
  ;[1 1 1] 检测任务状态
  (if (CallFunction|IsOpenedTask)
    (if (and (== (Variables|Default|GetChildTask_Count) (Variables|Default|GetCompletedChildTask_Count)) (== (Variables|Default|GetCompletedTaskItems_Count) (Variables|Default|GetTaskItem_Count)))
      (Variables|Config|SetTaskState "NewEnumerator2")
      (else
        (Variables|Config|SetTaskState "NewEnumerator1")))))

(event Custom|AddChildTask
  (params (Task :type BP%20Task%20Base%20Object%20Reference))
  ;[1 1 1] 添加子任务
  (Utilities|Array|AddUnique (Variables|Config|GetChildTasks) Task)
  (Variables|Default|SetChildTask_Count (Utilities|Array|Length (Variables|Config|GetChildTasks))))

(event Custom|ChangeTaskItemRunningState
  (params (IsFinished :type ETaskItemRunningState%20Enum) (TaskItem :type BP%20Task%20Item%20Base%20Object%20Reference))
  ;[1 1 1] 有任务物品完成任务，更新状态
  (if (CallFunction|IsOpenedTask)
    (CallFunction|NotifyChangeTaskItemRunningState IsFinished TaskItem)))

(event Custom|RelatedTaskOpenCheck
  ;[1 1 1] 关联任务开启时，先做自检
  (if (Utilities|Enum|Equal(Enum) (Variables|Config|GetTaskState) "NewEnumerator0")
    (Variables|Config|SetTaskState "NewEnumerator1")
    (CallFunction|CheckChildTaskFinished)
    (CallFunction|CalculateCompletedTaskItemCount)))

(event Custom|NotifyChangeTaskItemRunningState
  (params (IsFinished :type ETaskItemRunningState%20Enum) (TaskItem :type BP%20Task%20Item%20Base%20Object%20Reference))
  ;[1 1 1] 有任务物品完成任务，更新状态
  (switch Utilities|FlowControl|Switch|SwitchonETaskItemRunningState IsFinished
    (:NewEnumerator2
      (CallFunction|CalculateCompletedTaskItemCount))))

(event EventBeginPlay
  ;[1 1 1] BeginPlay
  (Utilities|FlowControl|Sequence
    (:then_0
      (CallFunction|InitTaskData))))

(fn ConstructionScript)

(fn OnRepTaskState
  (switch Utilities|FlowControl|Switch|SwitchonETaskState (Variables|Config|GetTaskState)
    (:NewEnumerator2
      (Utilities|FlowControl|Sequence
        (:then_0
          ;[1 1 1] 完成任务后，对任务物品进行处理
          (for _array_element (Variables|Config|GetTaskItems)
            (Default|TaskNotifytoDo _array_element))
          ;[1 1 1] Debug
          (Development|PrintString (Utilities|String|Append (Variables|Config|GetTaskName) ":" "Finished!") true true "(R=1.000000,G=0.231797,B=0.000000,A=1.000000)" 2e+02))
        (:then_1
          ;[1 1 1] 通知父任务更新状态
          (for _array_element_2 (Variables|Config|GetParentTasks)
            (CallFunction|CheckChildTaskFinished _array_element_2)))
        (:then_2
          ;[1 1 1] 全局广播任务完成
          (Default|CallTaskFinished (.AsGS%20VR (Utilities|Casting|CastToGS_VR (Game|GetGameState))) (Variables|Config|GetTaskName)))
        (:then_3
          ;[1 1 1] 开启关联任务
          (for _array_element_3 (Variables|Config|GetRelatedTask)
            (CallFunction|RelatedTaskOpenCheck _array_element_3)))))))

(fn IsOpenedTask
  (if (Utilities|Enum|Equal(Enum) (Variables|Config|GetTaskState) "NewEnumerator1")
    (return true)
    (else
      (return false))))