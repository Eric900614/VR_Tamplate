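; BP_TaskItemBase is a base Blueprint for task items that track a replicated running state and report it to an owning task.
; The owner task is set through a ServerSetOwner to NotifySetOwner event pair.
; When the state's RepNotify sees Completed while the owner task is open, NotifyTask passes the state and item to that task.
; TaskNotifytoDo hands the item and its finished to-do setting to a shared helper function.
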(event Custom|ServerSetOwner
  (params (Task :type BP%20Task%20Base%20Object%20Reference))
  ;[1 1 1] Set Owner Task
  (CallFunction|NotifySetOwner Task))

(event Custom|ChangeTaskItemState
  (params (ItemState :type ETaskItemRunningState%20Enum))
  ;[1 1 1] 更改任务物品状态
  (Variables|Config|Task|SetTaskItemRunningState ItemState))

(event Custom|NotifySetOwner
  (params (Task :type BP%20Task%20Base%20Object%20Reference))
  ;[1 1 1] Set Owner Task
  (Variables|Config|Task|SetOwnerTask Task))

(event EventTaskNotifytoDo
  ;[1 1 1] Task Item Interface Func
  (CallFunction|BPFTaskNotifyItemtoDo (Variables|Config|Task|GetTaskFinishedToDo) self (Utilities|Array|MakeArray 0)))

(event EventNotifyTask
  (bind _ownertask (Variables|Config|Task|GetOwnerTask))
  ;[1 1 1] Task Item Interface Func
  (Utilities|IsValid _ownertask
    (:Is%20Valid
      (Default|ChangeTaskItemRunningState _ownertask (Variables|Config|Task|GetTaskItemRunningState) self))))

(fn ConstructionScript)

(fn OnRepTaskItemRunningState
  (bind _ownertask (Variables|Config|Task|GetOwnerTask))
  (Utilities|IsValid _ownertask
    (:Is%20Valid
      (if (Default|IsOpenedTask _ownertask)
        (switch Utilities|FlowControl|Switch|SwitchonETaskItemRunningState (Variables|Config|Task|GetTaskItemRunningState)
          (:NewEnumerator2
            (CallFunction|NotifyTask)))))))